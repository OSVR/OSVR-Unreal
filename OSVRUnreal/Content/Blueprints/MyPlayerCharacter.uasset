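; Player character Blueprint that drives a left hand from OSVR tracking and reports OSVR button input.
; On BeginPlay it binds a handler to the OSVR input's button-state event, which prints a debug message on screen for each change.
; Every Tick it reads the left-hand interface position and rotation and applies them as HandLeft's relative transform, without sweep.
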(event Custom|OnButtonStateChanged_Event_0
  (params (Name :type Name :default "None") (State :type EButtonState%20Enum :default "PRESSED"))
  ;[1 1 1] Event handler on button inputs
  (Development|PrintString (Utilities|String|ToString(Text) (Utilities|Text|FormatText "Button: \"name\" [{status}]" (Utilities|Text|ToText(Name) Name) (Utilities|Text|ToText(String) (Utilities|String|ToString(Byte) State)))) true false))

(event EventTick
  (params (DeltaSeconds :type Float%20%28single-precision%29))
  ;[1 1 1] Apply roto-translations at each tick.
  (bind _returnvalue (Class|OSVRBPFunctionLibrary|GetInterfacePosition "/me/hands/left"))
  (bind _returnvalue_2 (Class|OSVRBPFunctionLibrary|GetInterfaceRotation "/me/hands/left"))
  (Transformation|SetRelativeLocationAndRotation (Variables|Default|GethandLeft) _returnvalue _returnvalue_2 false))

(event EventBeginPlay
  ;[1 1 1] Initialize events binding
  (EventDispatchers|BindEventtoOnButtonStateChanged (Variables|Default|GetOSVRInput) (delegate Custom|OnButtonStateChanged_Event_0)))

(fn ConstructionScript)